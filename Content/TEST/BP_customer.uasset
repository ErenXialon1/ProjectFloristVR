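; Customer character for a florist game that starts the BT_Customer behavior tree on its AI controller at BeginPlay.
; On overlapping a customerPoint, it rolls random wants for five occasion categories (love, sorrow, gift, celebration, apology) and shows them on text components.
; Only the love, sorrow and gift rolls reach the Wantings array; celebration and apology store zero while displaying their rolls.
; A helper hides the texts; debug prints remain.
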(event `self.ReceiveBeginPlay`
  (bind _ascustomer_aicontroller (cast `/Game/TEST/customerAIController` (`AIBlueprintHelperLibrary.GetAIController` self)))
  (`AIController.RunBehaviorTree` _ascustomer_aicontroller "/Game/TEST/BT_Customer.BT_Customer")
  (`KismetSystemLibrary.PrintString` "a")
  (bind _asproject_florist_gm (cast `/Game/TEST/ProjectFlorist_GM` (`GameplayStatics.GetGameMode`)))
  (set `self.As Project Florist GM` _asproject_florist_gm))

(event `self.ReceiveActorBeginOverlap`
  (params (OtherActor :type "Actor Object Reference"))
  (cast `/Game/TEST/customerPoint` OtherActor)
  (`KismetSystemLibrary.PrintString` "accessed customer point")
  (`self.setWantings`)
  (`self.printWantings`))

(event `self.ReceiveTick`
  (params (DeltaSeconds :type "Float (single-precision)")))

(fn `addArrayItems`)

(fn `nonVisibleWantings`
  (`SceneComponent.SetVisibility` (`self.ÖzürText`) false false)
  (`SceneComponent.SetVisibility` (`self.KutlamaText1`) false false)
  (`SceneComponent.SetVisibility` (`self.HediyeText1`) false false)
  (`SceneComponent.SetVisibility` (`self.HüzünText1`) false false)
  (`SceneComponent.SetVisibility` (`self.AşkText1`) false false)
  (`SceneComponent.SetVisibility` (`self.ÖzürText1`) false false)
  (`SceneComponent.SetVisibility` (`self.HediyeText`) false false)
  (`SceneComponent.SetVisibility` (`self.KutlamaText`) false false)
  (`SceneComponent.SetVisibility` (`self.HüzünText`) false false)
  (`SceneComponent.SetVisibility` (`self.AşkText`) false false))

(fn `printWantings`
  (`SceneComponent.SetVisibility` (`self.ÖzürText`) true false)
  (`SceneComponent.SetVisibility` (`self.KutlamaText1`) true false)
  (`SceneComponent.SetVisibility` (`self.HediyeText1`) true false)
  (`SceneComponent.SetVisibility` (`self.HüzünText1`) true false)
  (`SceneComponent.SetVisibility` (`self.AşkText1`) true false)
  (`SceneComponent.SetVisibility` (`self.ÖzürText1`) true false)
  (`SceneComponent.SetVisibility` (`self.HediyeText`) true false)
  (`SceneComponent.SetVisibility` (`self.KutlamaText`) true false)
  (`SceneComponent.SetVisibility` (`self.HüzünText`) true false)
  (`SceneComponent.SetVisibility` (`self.AşkText`) true false))

(fn `setWantings`
  (bind _output_get (set `self.wantingAşk` (`KismetMathLibrary.RandomIntegerInRange` 0 5)))
  (`KismetArrayLibrary.Array_Add` (`self.wantings`) _output_get)
  (`TextRenderComponent.K2_SetText` (`self.AşkText`) (`KismetTextLibrary.Conv_IntToText` _output_get))
  (bind _output_get_2 (set `self.wantingHüzün` (`KismetMathLibrary.RandomIntegerInRange` 0 5)))
  (`KismetArrayLibrary.Array_Add` (`self.wantings`) _output_get_2)
  (`TextRenderComponent.K2_SetText` (`self.HüzünText`) (`KismetTextLibrary.Conv_IntToText` _output_get_2))
  (bind _output_get_3 (set `self.wantingHediye` (`KismetMathLibrary.RandomIntegerInRange` 0 5)))
  (`KismetArrayLibrary.Array_Add` (`self.wantings`) _output_get_3)
  (`TextRenderComponent.K2_SetText` (`self.HediyeText`) (`KismetTextLibrary.Conv_IntToText` _output_get_3))
  (bind _output_get_4 (set `self.wantingKutlama` (`KismetMathLibrary.RandomIntegerInRange` 0 5)))
  (`KismetArrayLibrary.Array_Add` (`self.wantings`))
  (`TextRenderComponent.K2_SetText` (`self.KutlamaText`) (`KismetTextLibrary.Conv_IntToText` _output_get_4))
  (bind _output_get_5 (set `self.wantingÖzür` (`KismetMathLibrary.RandomIntegerInRange` 0 5)))
  (`KismetArrayLibrary.Array_Add` (`self.wantings`))
  (`TextRenderComponent.K2_SetText` (`self.ÖzürText`) (`KismetTextLibrary.Conv_IntToText` _output_get_5)))

(fn `UserConstructionScript`)